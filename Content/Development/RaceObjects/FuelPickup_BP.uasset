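; FuelPickup_BP is a pickup that adds ammo to the player, despite its fuel name and health comment.
; On ThirdPersonCharacter overlap it deactivates, adds WeaponChargeBonus to CurrentClipAmmo if below max, updates MyPlayerController's ammo text and destroys itself.
; The bonus can overshoot the max; otherwise ammo is set to max, but the text still adds the bonus.
; BeginPlay sets a fixed rotation once; Tick is empty.
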(event EventBeginPlay
  ;[1 1 1] Rotate Mesh
  (Transformation|SetActorRotation "1.000000, 0, 0"))

(event Collision|EventActorBeginOverlap
  (params (OtherActor :type Actor%20Object%20Reference))
  ;[1 1 1] Add Health when overlapped
  (bind _asthird_person_character (Utilities|Casting|CastToThirdPersonCharacter OtherActor))
  (Class|Pickup|SetActive false)
  (bind _asmy_player_controller (Utilities|Casting|CastToMyPlayerController (Pawn|GetController _asthird_person_character)))
  (if (< (Variables|/Game/Development/MechRacerBP/ThirdPersonBP/Blueprints/ThirdPersonCharacter.ThirdPersonCharacter_C|GetCurrentClipAmmo _asthird_person_character) (Variables|/Game/Development/MechRacerBP/ThirdPersonBP/Blueprints/ThirdPersonCharacter.ThirdPersonCharacter_C|GetMaxClipAmmo _asthird_person_character))
    (bind _output_get (Variables|/Game/Development/MechRacerBP/ThirdPersonBP/Blueprints/ThirdPersonCharacter.ThirdPersonCharacter_C|SetCurrentClipAmmo _asthird_person_character (+ (Variables|Default|GetWeaponChargeBonus) (Variables|/Game/Development/MechRacerBP/ThirdPersonBP/Blueprints/ThirdPersonCharacter.ThirdPersonCharacter_C|GetCurrentClipAmmo _asthird_person_character))))
    (Variables|/Game/Development/CheckpointSystem/MyPlayerController.MyPlayerController_C|SetCurrentAmmoText _asmy_player_controller (Utilities|Text|ToText(Integer) _output_get))
    (else
      (Variables|/Game/Development/MechRacerBP/ThirdPersonBP/Blueprints/ThirdPersonCharacter.ThirdPersonCharacter_C|SetCurrentClipAmmo _asthird_person_character (Variables|/Game/Development/MechRacerBP/ThirdPersonBP/Blueprints/ThirdPersonCharacter.ThirdPersonCharacter_C|GetMaxClipAmmo _asthird_person_character))
      (Variables|/Game/Development/CheckpointSystem/MyPlayerController.MyPlayerController_C|SetCurrentAmmoText _asmy_player_controller (Utilities|Text|ToText(Integer) (+ (Variables|Default|GetWeaponChargeBonus) (Variables|/Game/Development/MechRacerBP/ThirdPersonBP/Blueprints/ThirdPersonCharacter.ThirdPersonCharacter_C|GetCurrentClipAmmo _asthird_person_character))))))
  (Actor|DestroyActor))

(event EventTick
  (params (DeltaSeconds :type Float%20%28single-precision%29)))

(fn ConstructionScript)