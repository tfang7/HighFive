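; Health pickup actor for the race mode that adds a bonus to the player's mech health on overlap.
; It sets a fixed tilted rotation at begin play and calls SetActive(false) on any overlap, before casting to ThirdPersonCharacter and MyPlayerController.
; The health check looks inverted: HealthBonus is added, the actor destroyed and the total printed only when current health is at or above maximum.
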(event EventBeginPlay
  ;[1 1 1] Rotate Mesh
  (Transformation|SetActorRotation "10.000000,10.000000,10.000000"))

(event EventActorBeginOverlap
  (params (OtherActor :type Actor%20Object%20Reference))
  ;[1 1 1] Add Health when overlapped
  (CallFunction|SetActive false)
  (bind _asthird_person_character (Utilities|Casting|CastToThirdPersonCharacter OtherActor))
  (bind _asmy_player_controller (Utilities|Casting|CastToMyPlayerController (Game|GetPlayerController _asthird_person_character)))
  (if (not (< (Variables|/Game/Development/CheckpointSystem/MyPlayerController.MyPlayerController_C|GetCurrentMechHealth _asmy_player_controller) (Variables|/Game/Development/CheckpointSystem/MyPlayerController.MyPlayerController_C|GetMaxMechHealth _asmy_player_controller)))
    (bind _output_get (Variables|/Game/Development/CheckpointSystem/MyPlayerController.MyPlayerController_C|SetCurrentMechHealth _asmy_player_controller (+ (Variables|Default|GetHealthBonus) (Variables|/Game/Development/CheckpointSystem/MyPlayerController.MyPlayerController_C|GetCurrentMechHealth _asmy_player_controller))))
    (Actor|DestroyActor)
    (Development|PrintString (Utilities|String|ToString(Float) _output_get))))

(event EventTick
  (params (DeltaSeconds :type Float%20%28single-precision%29)))

(fn ConstructionScript)