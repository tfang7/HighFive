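; BP_BoostPad is a race pad that pushes and heals third-person characters inside its box.
; Each tick it updates their health, flags them as boosted and offsets them along the arrow's direction by Speed.
; A DoOnce adds a one-off burst offset, and ending overlap clears the boosted flag and resets it.
; The construction script counters actor scale on the arrow.
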(event Custom|OnComponentEndOverlap_Event_0
  (params (OtherActor :type Actor%20Object%20Reference) (OtherComp :type Primitive%20Component%20Object%20Reference) (OtherBodyIndex :type Integer))
  ;[1 1 1] Reset boost on leave and reset boosted bool
  (bind _asthird_person_character (Utilities|Casting|CastToThirdPersonCharacter OtherActor))
  (Variables|/Game/Development/MechRacerBP/ThirdPersonBP/Blueprints/ThirdPersonCharacter.ThirdPersonCharacter_C|SetisBoosted _asthird_person_character false)
  ;[1 1 1] Boost Mech when overlapping
  (Utilities|FlowControl|DoOnce false) ; enters at Reset
)

(event EventBeginPlay)

(event EventActorBeginOverlap
  (params (OtherActor :type Actor%20Object%20Reference)))

(event EventTick
  (params (DeltaSeconds :type Float%20%28single-precision%29))
  (bind _arrow (Variables|Default|GetArrow))
  (bind _returnvalue (Math|Vector|GetForwardVector _arrow))
  ;[1 1 1] Boost Mech when overlapping
  (for _array_element (Collision|GetOverlappingActors (Variables|Default|GetBox) "/Game/Development/MechRacerBP/ThirdPersonBP/Blueprints/ThirdPersonCharacter.ThirdPersonCharacter_C" :!class /Script/Engine.PrimitiveComponent)
    (bind _asthird_person_character (Utilities|Casting|CastToThirdPersonCharacter _array_element))
    (Default|UpdateHealth _asthird_person_character (Variables|Default|GetHealAmount))
    (Variables|/Game/Development/MechRacerBP/ThirdPersonBP/Blueprints/ThirdPersonCharacter.ThirdPersonCharacter_C|SetisBoosted _asthird_person_character true)
    (Transformation|AddActorWorldOffset _asthird_person_character (* (* _returnvalue (Variables|Default|GetSpeed)) DeltaSeconds))
    (Utilities|FlowControl|DoOnce false
      (:Completed
        (Transformation|AddActorWorldOffset _asthird_person_character (* _returnvalue (Variables|Default|GetBurstSpeed)))))))

(event EventBeginPlay
  ;[1 1 1] Reset boost on leave and reset boosted bool
  (Collision|AssignOnComponentEndOverlap (Variables|Default|GetBox) (delegate Custom|OnComponentEndOverlap_Event_0)))

(fn ConstructionScript
  (Transformation|SetRelativeScale3D (Variables|Default|GetArrow) (/ "1.000000,1.000000,1.000000" (Transformation|GetActorScale3D))))